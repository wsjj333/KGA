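; Player pawn that moves on its root's up/right plane and fires bullets from an arrow component.
; On BeginPlay it jumps to a fixed start location and plays a sound.
; Tick applies normalized, swept movement and, while Space is held, spawns BP_Bullet every frame with no cooldown until the ammo counter hits its limit.
; Pressing R resets the counter to reload; the IsWall check is always true.
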(event `self.ReceiveBeginPlay`
  (`SceneComponent.K2_SetWorldLocation` (`self.DefaultSceneRoot`) (-1000.0 -800.0 71.0) false false)
  (`GameplayStatics.PlaySound2D` "/Game/ShootingSource/Sound/action.action" 1.0 1.0 0.0 null null))

(event `self.ReceiveTick`
  (params (DeltaSeconds :type "Float (single-precision)"))
  (bind _ammo (`self.Ammo`))
  (bind (_returnvalue_location _returnvalue_rotation) (`KismetMathLibrary.BreakTransform` (`SceneComponent.K2_GetComponentToWorld` (`self.Arrow`))))
  ;[1 1 1] Player Move
  (bind _output_get (set `self.ForwardAxis` (`self.GetInputAxisValue`)))
  (bind _output_get_2 (set `self.RightAxis` (`self.GetInputAxisValue`)))
  (set `self.isWall` true)
  (if (`self.isWall`)
    (`self.K2_AddActorWorldOffset` (* (`KismetMathLibrary.Normal` (+ (* _output_get_2 (`SceneComponent.GetRightVector` (`self.DefaultSceneRoot`))) (* _output_get (`SceneComponent.GetUpVector` (`self.DefaultSceneRoot`))))) (* DeltaSeconds (`self.Speed`))) true)
    (bind _output_get_3 (set `self.IsFire` (`PlayerController.IsInputKeyDown` (`GameplayStatics.GetPlayerController` 0) "SpaceBar")))
    (if _output_get_3
      (if (not (`self.isAmmoOver`))
        (`|SpawnActorFromClass` "/Game/Player/BP_Bullet.BP_Bullet_C" (`KismetMathLibrary.MakeTransform` _returnvalue_location _returnvalue_rotation) "Undefined" "MultiplyWithRoot" null null)
        (`GameplayStatics.PlaySound2D` "/Game/ShootingSource/Sound/Shot.Shot" 1.0 1.0 0.0 null null)
        (`KismetSystemLibrary.PrintText` (`KismetTextLibrary.Conv_IntToText` _ammo))
        (set `self.Ammo` (+ _ammo 1))
        (set `self.isAmmoOver` (== (`self.Ammo`) 6))))))

(event `Key|R`
  (params (Key :type "Key Structure"))
  ;[1 1 1] Reload
  (:`Pressed`
    (set `self.Ammo` 1)
    (set `self.isAmmoOver` false)
    (`KismetSystemLibrary.PrintText` "리로드 완료!")))

(fn `UserConstructionScript`)
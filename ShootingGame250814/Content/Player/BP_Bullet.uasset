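; Bullet projectile actor that serves both player and enemy factions and deals point damage to actors it overlaps.
; On BeginPlay, Faction selects the Box's collision profile and the trace channel it ignores, then launches the Bullet component forward with a velocity-change impulse.
; Box overlaps apply Damage using the bullet's velocity as hit direction and its instigator's controller, without destroying the bullet.
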(event `self.ReceiveBeginPlay`
  (switch `/Game/E_Faction` (`self.Faction`)
    (:`NewEnumerator0`
      (`PrimitiveComponent.SetCollisionProfileName` (`self.Box`) "PlayerPreset" true)
      (`PrimitiveComponent.SetCollisionResponseToChannel` (`self.Box`) "ECC_GameTraceChannel1" "ECR_Ignore")
      (`PrimitiveComponent.IgnoreActorWhenMoving` (`self.Box`) null true)
      (`PrimitiveComponent.AddImpulse` (`self.Bullet`) (* (`self.GetActorForwardVector`) 1000.0) "None" true))
    (:`NewEnumerator1`
      (`PrimitiveComponent.SetCollisionProfileName` (`self.Box`) "EnemeyPreset" true)
      (`PrimitiveComponent.SetCollisionResponseToChannel` (`self.Box`) "ECC_GameTraceChannel2" "ECR_Ignore")
      (`PrimitiveComponent.IgnoreActorWhenMoving` (`self.Box`) null true)
      (`PrimitiveComponent.AddImpulse` (`self.Bullet`) (* (`self.GetActorForwardVector`) 1000.0) "None" true))))

(event `self.Box.OnComponentBeginOverlap`
  (params (OverlappedComponent :type "PrimitiveComponent Object Reference") (OtherActor :type "Actor Object Reference") (OtherComp :type "PrimitiveComponent Object Reference") (OtherBodyIndex :type Integer) (bFromSweep :type Boolean) (SweepResult :type "HitResult Structure (by ref)"))
  (`GameplayStatics.ApplyPointDamage` OtherActor (`self.Damage`) (`self.GetVelocity`) SweepResult (`self.GetInstigatorController`) self))

(fn `UserConstructionScript`)
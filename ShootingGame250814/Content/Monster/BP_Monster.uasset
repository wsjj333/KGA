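; BP_Monster is an enemy that moves along negative X while spinning a cube, fires bullets, and despawns past a fixed X limit.
; Tick updates its widget health bar and uses a Delay as the fire-rate gate for spawning BP_Bullet from the Arrow.
; Overlapping bullets are destroyed, while point damage lowers health and triggers the Die dispatcher at zero.
; The death handler passes experience to the player's BP_Pawn via LevelUp, then destroys the monster.
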(event `self.ReceiveBeginPlay`
  (set `self.M_hp` (`self.M_Maxhp`))
  (add `self.Die` (delegate `Die_Event`)))

(event `Die_Event`
  (set `self.bDead` true)
  (`self.SetActorTickEnabled` true)
  (`PrimitiveComponent.SetCollisionEnabled` (`self.Box`) "PhysicsOnly")
  (bind _asbp_pawn (cast `/Game/Player/BP_Pawn` (`GameplayStatics.GetPlayerPawn` 0)))
  (`/Game/Player/BP_Pawn.LevelUp` _asbp_pawn (`self.e_Exp`))
  (`self.K2_DestroyActor`))

(event `self.ReceiveActorBeginOverlap`
  (params (OtherActor :type "Actor Object Reference"))
  (bind _asbp_bullet (cast `/Game/Player/BP_Bullet` OtherActor))
  (`self.K2_DestroyActor` _asbp_bullet))

(event `self.ReceiveTick`
  (params (DeltaSeconds :type "Float (single-precision)"))
  (bind (_returnvalue_location _returnvalue_rotation) (`KismetMathLibrary.BreakTransform` (`SceneComponent.K2_GetComponentToWorld` (`self.Arrow`))))
  (bind _asmonster_hp (cast `/Game/Player/MonsterHp` (`WidgetComponent.GetUserWidgetObject` (`self.WBP_Monster`))))
  ;[1 1 1] Monster Move & destroy
  (`/Game/Player/MonsterHp.SetHpBar` _asmonster_hp (`self.M_Maxhp`) (`self.M_hp`))
  (if (not (`self.bDead`))
    (`self.K2_AddActorWorldOffset` (`KismetMathLibrary.MakeVector` (- 0.0 (* DeltaSeconds (`self.M_Speed`)))) true)
    (`SceneComponent.K2_AddWorldRotation` (`self.Cube3`) (`KismetMathLibrary.MakeRotator` 0.0 (* DeltaSeconds 200.0)) false false)
    (`KismetSystemLibrary.Delay` 0.25)
    (`|SpawnActorFromClass` "/Game/Player/BP_Bullet.BP_Bullet_C" (`KismetMathLibrary.MakeTransform` _returnvalue_location _returnvalue_rotation (2.0 2.0 2.0)) "Undefined" "MultiplyWithRoot" self 5.0 "NewEnumerator1" (`GameplayStatics.GetPlayerPawn` 0))
    (`PrimitiveComponent.SetCollisionObjectType` (`self.Box`) "ECC_GameTraceChannel2")
    (`self.SetOwner` null)
    (if (<= (.x (`self.K2_GetActorLocation`)) -1000.0)
      (`self.K2_DestroyActor`))))

(event `self.ReceivePointDamage`
  (params (Damage :type "Float (single-precision)") (DamageType :type "DamageType Object Reference") (HitLocation :type "Vector Structure") (HitNormal :type "Vector Structure") (HitComponent :type "PrimitiveComponent Object Reference") (BoneName :type Name) (ShotFromDirection :type "Vector Structure") (InstigatedBy :type "Controller Object Reference") (DamageCauser :type "Actor Object Reference") (HitInfo :type "HitResult Structure (by ref)"))
  (bind _returnvalue (`KismetMathLibrary.FClamp` (- (`self.M_hp`) Damage) 0.0 (`self.M_Maxhp`)))
  (set `self.LastImpact` HitLocation)
  (if (not (`self.bDead`))
    (set `self.M_hp` _returnvalue)
    (if (<= _returnvalue 0.0)
      (`self.Die`))))

(fn `UserConstructionScript`)